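; BP_platform-move is a platform whose Plane slides between its starting position and an End marker when the third-person character triggers it.
; BeginPlay caches the relative locations of Plane and End.
; Overlapping Box plays a timeline that lerps Plane between them, without sweep.
; Reversal is triggered by the character ending overlap with the End component, rather than with Box.
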(event OnComponentBeginOverlap(Box)
  (params (OverlappedComponent :type Primitive%20Component%20Object%20Reference) (OtherActor :type Actor%20Object%20Reference) (OtherComp :type Primitive%20Component%20Object%20Reference) (OtherBodyIndex :type Integer) (bFromSweep :type Boolean) (SweepResult :type Hit%20Result%20Structure%20%28by%20ref%29))
  (Utilities|Casting|CastToThirdPersonCharacter OtherActor)
  (bind _newtrack_0 (Timeline|Timeline_0 Play)
    (:Update
      (Transformation|SetRelativeLocation (Variables|Default|GetPlane) (Math|Vector|Lerp(Vector) (Variables|Default|Getstart%20loc) (Variables|Default|Getend%20loc) _newtrack_0) false false))))

(event OnComponentEndOverlap(end)
  (params (OverlappedComponent :type Primitive%20Component%20Object%20Reference) (OtherActor :type Actor%20Object%20Reference) (OtherComp :type Primitive%20Component%20Object%20Reference) (OtherBodyIndex :type Integer))
  (Utilities|Casting|CastToThirdPersonCharacter OtherActor)
  (bind _newtrack_0 (Timeline|Timeline_0 Reverse)
    (:Update
      (Transformation|SetRelativeLocation (Variables|Default|GetPlane) (Math|Vector|Lerp(Vector) (Variables|Default|Getstart%20loc) (Variables|Default|Getend%20loc) _newtrack_0) false false))))

(event EventBeginPlay
  (Variables|Default|Setstart%20loc (Variables|/Script/Engine.SceneComponent|GetRelativeLocation (Variables|Default|GetPlane)))
  (Variables|Default|Setend%20loc (Variables|/Script/Engine.SceneComponent|GetRelativeLocation (Variables|Default|Getend))))

(fn ConstructionScript)